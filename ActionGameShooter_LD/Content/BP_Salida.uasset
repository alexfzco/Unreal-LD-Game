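; BP_Salida is an exit actor that removes itself once no BP_IAEnemigoSimple enemies remain in the level.
; On BeginPlay it creates a WBP_Aviso notice widget and starts a looping one-second timer.
; Each tick of the timer polls for remaining enemies; when none are found it shows the widget on screen and destroys the actor.
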(event `self.ReceiveBeginPlay`
  (bind _returnvalue (`|CreateWidget` "/Game/Variant_Shooter/Blueprints/WBP_Aviso.WBP_Aviso_C"))
  (set `self.Aviso_WBP` _returnvalue)
  (`KismetSystemLibrary.K2_SetTimerDelegate` (delegate `CE_Destruir`) 1.0 true))

(event `CE_Destruir`
  (bind _outactors (`GameplayStatics.GetAllActorsOfClass` "/Game/Variant_Shooter/Blueprints/BP_IAEnemigoSimple.BP_IAEnemigoSimple_C"))
  (if (== (`KismetArrayLibrary.Array_Length` _outactors) 0)
    (`UserWidget.AddToViewport` (`self.Aviso_WBP`) 0)
    (`self.K2_DestroyActor`)))

(fn `UserConstructionScript`)