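; Turret actor the player can enter and rotate with the mouse; no firing logic is present.
; A box overlap enables or disables input, and the interact action flip-flops between entering and exiting.
; Entering zeroes the shooter character's walk speed, hides its mesh and blends the view to the turret, while exiting reverses this.
; While possessed by flag only, with no pawn possession, mouse X yaws the static mesh.
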(event `self.ReceiveBeginPlay`
  (`SceneComponent.SetVisibility` (`self.Cube`) false false))

(event `EnhancedInput|/Game/Variant_Shooter/Input/Actions/IA_Ineract`
  (params (ActionValue :type Boolean) (ElapsedSeconds :type "Float (double-precision)") (TriggeredSeconds :type "Float (double-precision)") (InputAction :type "InputAction Object Reference" :default "/Game/Variant_Shooter/Input/Actions/IA_Ineract.IA_Ineract"))
  (bind _returnvalue (`GameplayStatics.GetPlayerController` 0))
  (:`Started`
    (bind _asbp_shooter_character (cast `/Game/Variant_Shooter/Blueprints/BP_ShooterCharacter` (stale `self.Box.OnComponentBeginOverlap` OtherActor)))
    ; Entra en la torreta
    (`/Engine/EditorBlueprintResources/StandardMacros.FlipFlop`
      (:`A`
        (bind _charactermovement (`Character.CharacterMovement` _asbp_shooter_character))
        (set `CharacterMovementComponent.MaxWalkSpeed` 0.0 _charactermovement)
        (bind _mesh (`Character.Mesh` _asbp_shooter_character))
        (`SceneComponent.SetVisibility` _mesh false true)
        (`PlayerController.SetViewTargetWithBlend` _returnvalue self 0.2 "VTBlend_Linear" 0.0 false)
        (set `self.isPossesed` true))
      (:`B`
        ; Salir de la torreta
        (`PlayerController.SetViewTargetWithBlend` _returnvalue (`GameplayStatics.GetPlayerCharacter` 0) 0.2 "VTBlend_Linear" 0.0 false)
        (set `CharacterMovementComponent.MaxWalkSpeed` 600.0 _charactermovement)
        (`SceneComponent.SetVisibility` _mesh true true)
        (set `self.isPossesed` false)))))

(event `EnhancedInput|/Game/Input/Actions/IA_MouseLook`
  (params (ActionValue :type "Vector2D Structure") (ElapsedSeconds :type "Float (double-precision)") (TriggeredSeconds :type "Float (double-precision)") (InputAction :type "InputAction Object Reference" :default "/Game/Input/Actions/IA_MouseLook.IA_MouseLook"))
  ; Mira dentro de la torreta
  (:`Triggered`
    (if (`self.isPossesed`)
      (`SceneComponent.K2_AddWorldRotation` (`self.StaticMesh`) (`KismetMathLibrary.MakeRotator` 0.0 0.0 (* ActionValue_X 5.0)) false false))))

(event `self.Box.OnComponentBeginOverlap`
  (params (OverlappedComponent :type "PrimitiveComponent Object Reference") (OtherActor :type "Actor Object Reference") (OtherComp :type "PrimitiveComponent Object Reference") (OtherBodyIndex :type Integer) (bFromSweep :type Boolean) (SweepResult :type "HitResult Structure (by ref)"))
  ; Deja disparar
  (`self.EnableInput` null))

(event `self.Box.OnComponentEndOverlap`
  (params (OverlappedComponent :type "PrimitiveComponent Object Reference") (OtherActor :type "Actor Object Reference") (OtherComp :type "PrimitiveComponent Object Reference") (OtherBodyIndex :type Integer))
  ; No deja disparar
  (`self.DisableInput` null))

(fn `UserConstructionScript`)